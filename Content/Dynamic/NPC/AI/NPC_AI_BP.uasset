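; AI controller for guard NPCs that runs the GuardBehaviour tree on the PatrolData blackboard.
; AI perception stores any sensed actor without the "Guard" tag as the enemy key, and clears that key when such an actor is lost.
; Each tick, it turns the controlled Ue4ASP_Character's aiming and shooting flags on or off according to whether the controller has a valid focus actor.
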(event `self.ReceiveBeginPlay`
  (bind _blackboardcomponent (`self.UseBlackboard` "/Game/Dynamic/NPC/AI/PatrolData.PatrolData"))
  (set `self.BlackboardComponent` _blackboardcomponent)
  (`self.RunBehaviorTree` "/Game/Dynamic/NPC/AI/GuardBehaviour.GuardBehaviour"))

(event `self.ReceiveTick`
  (params (DeltaSeconds :type "Float (single-precision)"))
  (bind _returnvalue (`KismetSystemLibrary.IsValid` (`self.GetFocusActor`)))
  (bind _asue_4asp_character (cast `/Game/Dynamic/NPC/Behaviour/Ue4ASP_Character` (`self.K2_GetPawn`)))
  (set `/Game/Dynamic/NPC/Behaviour/Ue4ASP_Character.Aiming Behaviour` _returnvalue _asue_4asp_character)
  (set `/Game/Dynamic/NPC/Behaviour/Ue4ASP_Character.Shooting Behaviour` _returnvalue _asue_4asp_character))

(event `self.AIPerception.OnTargetPerceptionUpdated`
  (params (Actor :type "Actor Object Reference") (Stimulus :type "AIStimulus Structure"))
  (if (`self.ActorHasTag` Actor "Guard")
    _
    (elif (`.bSuccessfullySensed` (break `AIStimulus` Stimulus))
      (`BlackboardComponent.SetValueAsObject` (`self.BlackboardComponent`) (`self.AnemyKey`) Actor)
      (else
        (`BlackboardComponent.ClearValue` (`self.BlackboardComponent`) (`self.AnemyKey`))))))

(fn `UserConstructionScript`)