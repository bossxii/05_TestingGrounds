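; AI controller for guard NPCs that patrol and fight perceived enemies.
; On BeginPlay it sets up the PatrolData blackboard and runs the GuardBehaviour behavior tree.
; Perception updates store any sensed actor not tagged "Guard" as the blackboard enemy, clearing it when sensing fails.
; Each tick, the controlled character's aiming and shooting flags follow whether a focus actor is set.
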(event `self.ReceiveBeginPlay`
  ;[1 1 1] Set Blackboard and BehaviourTree
  (bind _blackboardcomponent (`self.UseBlackboard` "/Game/Dynamic/Character/AI/PatrolData.PatrolData"))
  (set `self.BlackboardComponent` _blackboardcomponent)
  (`self.RunBehaviorTree` "/Game/Dynamic/Character/AI/GuardBehaviour.GuardBehaviour"))

(event `self.ReceiveTick`
  (params (DeltaSeconds :type "Float (single-precision)"))
  (bind _returnvalue (`KismetSystemLibrary.IsValid` (`self.GetFocusActor`)))
  ;[1 1 1] Set Aiming & Shooting Behaviour
  (bind _ascharacter (cast `/Game/Dynamic/Character/Behaviour/Character` (`self.K2_GetPawn`)))
  (set `/Game/Dynamic/Character/Behaviour/Character.Aiming Behaviour` _returnvalue _ascharacter)
  (set `/Game/Dynamic/Character/Behaviour/Character.Shooting Behaviour` _returnvalue _ascharacter))

(event `self.AIPerception.OnTargetPerceptionUpdated`
  (params (Actor :type "Actor Object Reference") (Stimulus :type "AIStimulus Structure"))
  ;[1 1 1] Set Enemy from Perception
  (if (`self.ActorHasTag` Actor "Guard")
    _
    (elif (`.bSuccessfullySensed` (break `AIStimulus` Stimulus))
      (`BlackboardComponent.SetValueAsObject` (`self.BlackboardComponent`) (`self.AnemyKey`) Actor)
      (else
        (`BlackboardComponent.ClearValue` (`self.BlackboardComponent`) (`self.AnemyKey`))))))

(fn `UserConstructionScript`)